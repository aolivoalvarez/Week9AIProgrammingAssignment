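; Pong-style ball that bounces between the player paddle and an enemy paddle on the Y axis and off walls on Z.
; Paddle hits add randomized Z spin based on paddle move direction and raise max speed by a growing multiplier, with reversals debounced by a shared timer.
; Player hits also spawn an InvisiBallBP.
; Tick recenters the ball when it passes the player, resetting speed limits and destroying the latest InvisiBallBP.
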(event EventBeginPlay)

(event Collision|EventActorBeginOverlap
  (params (OtherActor :type Actor%20Object%20Reference))
  (bind _aspaddle_bp (Utilities|Casting|CastToPaddleBP OtherActor)
    (:then
      (CallFunction|HandleBounce (Variables|/Game/Blueprints/PaddleBP.PaddleBP_C|GetmoveDirection _aspaddle_bp))
      (bind _returnvalue (Game|SpawnActorfromClass "/Game/Blueprints/InvisiBallBP.InvisiBallBP_C" (Transformation|GetActorTransform) "AlwaysSpawn" 0 0)))
    (:CastFailed
      (bind _asenemy_bp (Utilities|Casting|CastToEnemyBP OtherActor)
        (:then
          (CallFunction|HandleBounce (Variables|/Game/Blueprints/EnemyBP.EnemyBP_C|GetmoveDirection _asenemy_bp)))
        (:CastFailed
          (Utilities|Casting|CastToWallBP OtherActor)
          (CallFunction|ReverseZ))))))

(event EventTick
  (params (DeltaSeconds :type Float%20%28single-precision%29))
  (bind _projectilemovement (Variables|Default|GetProjectileMovement))
  (Variables|Default|SettimeSinceReversed (+ DeltaSeconds (Variables|Default|GettimeSinceReversed)))
  (bind _outofbounds (CallFunction|IsOutOfBounds))
  (if _outofbounds
    (Transformation|SetActorLocation "0, 0, 0" false false)
    (Variables|/Script/Engine.MovementComponent|SetVelocity _projectilemovement (Math|Vector|MakeVector 0.0 (.Y (Math|Vector|BreakVector (Variables|/Script/Engine.MovementComponent|GetVelocity _projectilemovement))) 0.0))
    (Actor|DestroyActor (stale Collision|EventActorBeginOverlap _returnvalue))))

(fn ConstructionScript)

(fn IsOutOfBounds
  (bind _returnvalue (Transformation|GetActorLocation))
  (bind _y (Math|Vector|BreakVector _returnvalue))
  (bind _returnvalue_2 (Actor|GetActorOfClass "/Game/Blueprints/PaddleBP.PaddleBP_C"))
  (if (<= _y (.Y (Math|Vector|BreakVector (Transformation|GetActorLocation _returnvalue_2))))
    (Variables|Default|SetspeedMultiplier 1.0)
    (Variables|/Script/Engine.ProjectileMovementComponent|SetMaxSpeed (Variables|Default|GetProjectileMovement) 5e+02)
    (return true)
    (else
      (bind _returnvalue_3 (Actor|GetActorOfClass "/Game/Blueprints/EnemyBP.EnemyBP_C"))
      (if (not (>= _y (.Y (Math|Vector|BreakVector (Transformation|GetActorLocation _returnvalue_3)))))
        (return false)))))

(fn HandleBounce
  (params (Selection :type Integer))
  (bind _returnvalue (Math|Random|RandomFloatinRange -5e+01 5e+01))
  (switch int Selection
    (:-1
      (CallFunction|AddSpin (+ _returnvalue -125.0)))
    (:0
      (CallFunction|AddSpin (Math|Random|RandomFloatinRange -15.0 15.0)))
    (:1
      (CallFunction|AddSpin (+ _returnvalue 125.0))))
  (CallFunction|ReverseY))

(fn AddSpin
  (params (Spin :type Float%20%28single-precision%29))
  (bind _projectilemovement (Variables|Default|GetProjectileMovement))
  (Variables|/Script/Engine.MovementComponent|SetVelocity _projectilemovement (+ (Math|Vector|MakeVector 0.0 0.0 Spin) (Variables|/Script/Engine.MovementComponent|GetVelocity _projectilemovement))))

(fn ReverseY
  (bind _projectilemovement (Variables|Default|GetProjectileMovement))
  (if (>= (Variables|Default|GettimeSinceReversed) 1.0)
    (Variables|Default|SetspeedMultiplier (+ (Variables|Default|GetspeedMultiplier) 0.5))
    (Variables|/Script/Engine.ProjectileMovementComponent|SetMaxSpeed _projectilemovement (* (Variables|/Script/Engine.ProjectileMovementComponent|GetMaxSpeed _projectilemovement) (Variables|Default|GetspeedMultiplier)))
    (Variables|/Script/Engine.MovementComponent|SetVelocity _projectilemovement (Math|Vector|MakeVector (.X (Math|Vector|BreakVector (Variables|/Script/Engine.MovementComponent|GetVelocity _projectilemovement))) (* -1 (.Y (Math|Vector|BreakVector (Variables|/Script/Engine.MovementComponent|GetVelocity _projectilemovement)))) (.Z (Math|Vector|BreakVector (Variables|/Script/Engine.MovementComponent|GetVelocity _projectilemovement)))))
    (Variables|Default|SettimeSinceReversed 0.0)))

(fn ReverseZ
  (bind _projectilemovement (Variables|Default|GetProjectileMovement))
  (if (>= (Variables|Default|GettimeSinceReversed) 1.0)
    (Variables|/Script/Engine.MovementComponent|SetVelocity _projectilemovement (Math|Vector|MakeVector (.X (Math|Vector|BreakVector (Variables|/Script/Engine.MovementComponent|GetVelocity _projectilemovement))) (.Y (Math|Vector|BreakVector (Variables|/Script/Engine.MovementComponent|GetVelocity _projectilemovement))) (* -1 (.Z (Math|Vector|BreakVector (Variables|/Script/Engine.MovementComponent|GetVelocity _projectilemovement))))))
    (Variables|Default|SettimeSinceReversed 0.0)))