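; EnemyBP is an enemy actor that tracks the InvisiBallBP actor's height by moving up or down, like an AI paddle.
; Each Tick, it finds the invisible ball, and SetDirection compares Z positions to choose the movement sign.
; It then applies a swept local Z offset of MoveSpeed per frame, unscaled by delta time.
; If the ball cast fails, it only updates direction from PreviousPosition, without moving.
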(event EventBeginPlay)

(event Collision|EventActorBeginOverlap
  (params (OtherActor :type Actor%20Object%20Reference)))

(event EventTick
  (params (DeltaSeconds :type Float%20%28single-precision%29))
  ;[1 1 1] MovementBasedOnBall
  (bind _asinvisi_ball_bp (Utilities|Casting|CastToInvisiBallBPClass "/Game/Blueprints/InvisiBallBP.InvisiBallBP_C")
    (:then
      (bind _returnvalue (Actor|GetActorOfClass _asinvisi_ball_bp))
      (bind _output_get (Variables|Default|SettargetPosition (Transformation|GetActorLocation _returnvalue)))
      (CallFunction|SetDirection _output_get)
      (Transformation|AddActorLocalOffset (Math|Vector|MakeVector 0.0 0.0 (* (Variables|Default|GetmoveDirection) (Variables|Default|GetmoveSpeed))) true false))
    (:CastFailed
      (CallFunction|SetDirection (Variables|Default|GetpreviousPosition)))))

(fn ConstructionScript)

(fn SetDirection
  (params (position :type Vector))
  (bind _returnvalue (Transformation|GetActorLocation))
  (bind _z (Math|Vector|BreakVector position))
  (bind _z_2 (Math|Vector|BreakVector _returnvalue))
  (if (<= _z_2 _z)
    (Variables|Default|SetmoveDirection 1)
    (elif (>= _z_2 _z)
      (Variables|Default|SetmoveDirection -1)
      (else
        (Variables|Default|SetmoveDirection 0)))))